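; Spawner actor that produces a limited number of AI-controlled tanks at its location over the course of play.
; On BeginPlay it loops while SpawnCount remains, waiting a fixed delay before spawning each TankType, adjusted to avoid collisions.
; For each tank it spawns a TankAIController_BP, possesses the tank and sets the self and enemy camps on the controller's CampComponent.
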(event `self.ReceiveBeginPlay`
  (bind _spawncount (`self.SpawnCount`))
  (if (> _spawncount 0) :!label _label
    (set `self.SpawnCount` (- _spawncount 1))
    (`KismetSystemLibrary.Delay` 10.0)
    (bind _returnvalue (`|SpawnActorFromClass` (`self.TankType`) (`KismetMathLibrary.Conv_VectorToTransform` (`self.K2_GetActorLocation`)) "AdjustIfPossibleButAlwaysSpawn" "OverrideRootScale"))
    (bind _astank (cast `Tank` _returnvalue))
    (bind _returnvalue_2 (`|SpawnActorFromClass` "/Game/Blueprints/TankAIController_BP.TankAIController_BP_C" (`KismetMathLibrary.Conv_VectorToTransform` (`KismetMathLibrary.MakeVector` 0.0)) "Undefined" "OverrideRootScale"))
    (`Controller.Possess` _returnvalue_2 _astank)
    (bind _campcomponent (`/Game/Blueprints/TankAIController_BP.CampComponent` _returnvalue_2))
    (`CampComponent.SetSelfCamp` _campcomponent (`self.SelfCamp`))
    (`CampComponent.SetEnemyCamp` _campcomponent (`self.EnemyCamp`))
    (goto _label)))

(fn `UserConstructionScript`)